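; BP_WorldItem_Boost is a world item Blueprint for boost items, built on a parent that supplies base item data and pickup behavior.
; InitSpawnData looks up the spawn ID in DT_WorldItem_Boost, then fills the base type, name, UI prefix, mesh and icon and stores the unit weight.
; GetWeight multiplies that weight by Amount, and GetPickupData returns the parent's icon and name along with Amount.
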(fn `GetPickupData`
  (returns (ItemIcon :type "Texture2D Object Reference") (ItemName :type Text) (Amount :type Integer))
  (bind (_itemicon _itemname) (`parent.GetPickupData`))
  (return _itemicon _itemname (`self.Amount`)))

(fn `GetWeight`
  (returns (ReturnValue :type Integer))
  (return (* (`self.Amount`) (`self.SingleWeight`))))

(fn `InitSpawnData`
  (params (ID :type Name) (SN :type String))
  (`parent.InitSpawnData` ID SN)
  (bind _returnvalue (`|GetDataTableRow` "/Game/Blueprints/Datas/DataTable/Item/DT_WorldItem_Boost.DT_WorldItem_Boost" (`self.ID`))
    (:`then`
      (`self.InitWorldItemBaseData` (break `/Game/Blueprints/Datas/Struct/Item/ST_WorldItem_Useable` _returnvalue) (`.ItemName_14_E7B88F1C4959FCFDA6184CB292FCB78D` (break `/Game/Blueprints/Datas/Struct/Item/ST_WorldItem_Useable` _returnvalue)) (`.UIPrefix_9_98EC3BA34F7CD967D85839AD58ECA2C6` (break `/Game/Blueprints/Datas/Struct/Item/ST_WorldItem_Useable` _returnvalue)) (`.StaticMesh_27_078B116143ECCF337A8B83B0A3726DFF` (break `/Game/Blueprints/Datas/Struct/Item/ST_WorldItem_Useable` _returnvalue)) (`.ItemIcon_44_583B9A4446B4EDAFE64B9F97C61D1FAC` (break `/Game/Blueprints/Datas/Struct/Item/ST_WorldItem_Useable` _returnvalue)))
      (set `self.SingleWeight` (`.Weight_41_156DAC534731ABD139CA5F91C3F03746` (break `/Game/Blueprints/Datas/Struct/Item/ST_WorldItem_Useable` _returnvalue))))))

(fn `UserConstructionScript`
  (`parent.UserConstructionScript`))