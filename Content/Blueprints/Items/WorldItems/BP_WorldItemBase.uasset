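; BP_WorldItemBase is the base actor for items placed in the world.
; On BeginPlay it traces 1000 units down against the Land object type and moves itself to the hit location to sit on the ground.
; Init functions store spawn ID and SN, plus item type, name, UI prefix and static mesh.
; EnableOutline toggles the mesh's custom depth rendering for highlighting.
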(event `self.ReceiveBeginPlay`
  (bind (_returnvalue_x _returnvalue_y _returnvalue_z) (`KismetMathLibrary.BreakVector` (`self.K2_GetActorLocation`)))
  (`parent.ReceiveBeginPlay`)
  ; z축 -1000으로 레이져 쏜다 Land만 맞추겠다
  (bind _outhit (`KismetSystemLibrary.LineTraceSingleForObjects` (`self.K2_GetActorLocation`) (`KismetMathLibrary.MakeVector` _returnvalue_x _returnvalue_y (+ _returnvalue_z -1000.0)) (`|MakeArray` "ObjectTypeQuery7" :!type "EObjectTypeQuery Enum")))
  ; 부딪힌 곳으로 Set 시키기
  (`self.K2_SetActorLocation` (`.Location` (`GameplayStatics.BreakHitResult` _outhit))))

(fn `EnableOutline`
  (params (bIsEnabled :type Boolean))
  (`PrimitiveComponent.SetRenderCustomDepth` (`self.StaticMesh`) bIsEnabled))

(fn `InitSpawnData`
  (params (ID :type Name) (SN :type String))
  (set `self.ID` ID)
  (set `self.SN` SN))

(fn `InitWorldItemBaseData`
  (params (ItemType :type "/Game/Blueprints/Datas/Enum/Item/E_ItemType Enum" :default "NewEnumerator0") (ItemName :type Text) (UIPrefix :type "/Game/Blueprints/Datas/Enum/Item/E_UIPrefix Enum" :default "NewEnumerator0") (StataicMesh :type "StaticMesh Object Reference"))
  (set `self.ItemType` ItemType)
  (set `self.ItemName` ItemName)
  (set `self.UIPrefix` UIPrefix)
  (`StaticMeshComponent.SetStaticMesh` (`self.StaticMesh`) StataicMesh))

(fn `UserConstructionScript`
  (`parent.UserConstructionScript`))