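; Player character Blueprint handling movement, free look, pose and move states, and detection of nearby dropped items.
; Movement follows controller yaw, or actor yaw during free look, whose release eases the camera back through a timeline.
; Move state resolves by overwrite priority (aim, walk, run, default), and Tick broadcasts start/stop changes.
; Item detection filters a sphere trace by line of sight, broadcasting the set for UI when it changes.
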(event `self.ReceiveBeginPlay`
  (`KismetSystemLibrary.K2_SetTimerDelegate` (`|CreateDelegate` :!event `UpdateDroppedList`) 0.5 true))

(event `self.ReceiveTick`
  (params (DeltaSeconds :type "Float (single-precision)"))
  (bind _returnvalue (> (`KismetMathLibrary.VSizeSquared` (`self.GetVelocity`)) 0.0))
  (if (!= (`self.bIsMovingNow`) _returnvalue)
    (bind _output_get (set `self.bIsMovingNow` _returnvalue))
    (`self.OnMovementStateChange` _output_get)))

(event `OnFreeLookEnded`
  (bind (_direction _alpha) (`Timeline|Timeline` :!via `PlayFromStart`)
    (:`Update`
      (`Controller.SetControlRotation` (`self.GetController`) (`KismetMathLibrary.RLerp` (`self.FreeLookEndRotation`) (`self.FreeLookStartRotation`) _alpha true)))
    (:`Finished`
      (set `self.bUseControllerRotationYaw` true))))

(fn `EvaluateMoveState`
  ; 모든 조건 탐색 분기문
  (`|ExecutionSequence`
    (:`then_0`
      (set `self.CurrentMoveState` "NewEnumerator1"))
    (:`then_1`
      (if (`self.bIsRunPressed`)
        (set `self.CurrentMoveState` "NewEnumerator2")))
    (:`then_2`
      (if (`self.bIsWalkPressed`)
        (set `self.CurrentMoveState` "NewEnumerator0")))
    (:`then_3`
      (if (`self.bIsAimPressed`)
        (set `self.CurrentMoveState` "NewEnumerator3")))))

(fn `FreeLook`
  (params (bIsPressed :type Boolean))
  (bind _returnvalue (`self.GetControlRotation`))
  (if bIsPressed
    ; FreeLook 시작 회전값
    (set `self.FreeLookStartRotation` _returnvalue)
    (set `self.bUseControllerRotationYaw` false)
    (else
      ; FreeLook 끝 회전값
      (set `self.FreeLookEndRotation` _returnvalue)
      ; UseControllerRotationYaw True로 키는거 내부에 있음
      (`self.OnFreeLookEnded`))))

(fn `GetDroppedItems`
  (returns (ReturnDroppedItems :type "Set of Actor Object Reference"))
  (locals (ReturnDroppedItems :type "Set of Actor Object Reference"))
  (bind (_returnvalue_x _returnvalue_y _returnvalue_z) (`KismetMathLibrary.BreakVector` (`self.K2_GetActorLocation`)))
  (bind _returnvalue (`self.K2_GetActorLocation`))
  (bind _outhits (`KismetSystemLibrary.SphereTraceMultiForObjects` :`Start` _returnvalue :`End` _returnvalue :`Radius` 220.0 :`ObjectTypes` (`|MakeArray` "ObjectTypeQuery8" :!type "EObjectTypeQuery Enum") :`DrawTime` 2.0))
  (for _array_element _outhits
    (bind (_bblockinghit _binitialoverlap _time _distance _location _impactpoint _normal _impactnormal _physmat _hitactor) (`GameplayStatics.BreakHitResult` _array_element))
    (bind _outhit (`KismetSystemLibrary.LineTraceSingle` :`Start` (`KismetMathLibrary.MakeVector` _returnvalue_x _returnvalue_y (+ _returnvalue_z 80.0)) :`End` (`self.K2_GetActorLocation` _hitactor) :`TraceChannel` "TraceTypeQuery1" :`DrawDebugType` "ForDuration" :`DrawTime` 2.0))
    (bind (_bblockinghit_2 _binitialoverlap_2 _time_2 _distance_2 _location_2 _impactpoint_2 _normal_2 _impactnormal_2 _physmat_2 _hitactor_2) (`GameplayStatics.BreakHitResult` _outhit))
    (if (== _hitactor_2 _hitactor)
      (`BlueprintSetLibrary.Set_Add` (`local.ReturnDroppedItems`) _hitactor_2)))
  (return (`local.ReturnDroppedItems`)))

(fn `GetTargetRotationByControllerYaw`
  (returns (TargetRotation :type "Rotator Structure"))
  (return (`KismetMathLibrary.SelectRotator` (`/Game/Blueprints/Utils/MathUtils.GetYawOnlyRotation` (`self.GetControlRotation`)) (`/Game/Blueprints/Utils/MathUtils.GetYawOnlyRotation` (`self.K2_GetActorRotation`)) (`self.bUseControllerRotationYaw`))))

(fn `InputLookUp`
  (params (`Y Axis` :type "Float (double-precision)"))
  (`self.AddControllerPitchInput` `Y Axis`))

(fn `InputTurn`
  (params (`X Axis` :type "Float (double-precision)"))
  ; use controller Yaw를 true로 했기에
  ; 컨트롤러Yaw가 움직이는게 곧 플레이어Yaw가
  ; 움직이는 것이다
  (`self.AddControllerYawInput` `X Axis`))

(fn `Move`
  (params (bIsForward :type Boolean) (AxisValue :type "Float (double-precision)"))
  (bind _targetrotation (`self.GetTargetRotationByControllerYaw`))
  (if bIsForward
    (`self.AddMovementInput` (`KismetMathLibrary.GetForwardVector` _targetrotation) AxisValue)
    (else
      (`self.AddMovementInput` (`KismetMathLibrary.GetRightVector` _targetrotation) AxisValue))))

(fn `SetMaxWalkSpeed`
  (params (NewSpeed :type "Float (double-precision)"))
  (set `CharacterMovementComponent.MaxWalkSpeed` NewSpeed (`self.CharacterMovement`)))

(fn `UpdateDroppedList`
  (locals (OldDroppedItems :type "Set of Actor Object Reference") (NewDroppedItems :type "Set of Actor Object Reference") (bNeedUpdate :type Boolean))
  (set `local.OldDroppedItems` (`self.CurrentDroppedItmes`))
  (`|ExecutionSequence`
    (:`then_0`
      ; 길이 같은지 판단
      (bind _output_get (set `local.NewDroppedItems` (`self.GetDroppedItems`)))
      (if (== (`BlueprintSetLibrary.Set_Length` _output_get) (`BlueprintSetLibrary.Set_Length` (`local.OldDroppedItems`)))
        ; 내부 요소까지 같은지 확인
        (bind _valuepin (`|SetForEach` (`local.NewDroppedItems`) :!label _label)
          (:`then`
            (if (not (`BlueprintSetLibrary.Set_Contains` (`local.OldDroppedItems`) _valuepin))
              (set `local.bNeedUpdate` true)
              (goto _label :!via `BreakPin`))))
        (else
          (set `local.bNeedUpdate` true))))
    (:`then_1`
      (if (`local.bNeedUpdate`)
        (`BlueprintSetLibrary.Set_Clear` (`self.CurrentDroppedItmes`))
        (bind _valuepin_2 (`|SetForEach` (`local.NewDroppedItems`))
          (:`then`
            (bind _asbp_world_item_base (cast `/Game/Blueprints/Items/WorldItems/BP_WorldItemBase` _valuepin_2))
            ; Set 업데이트
            (`BlueprintSetLibrary.Set_Add` (`self.CurrentDroppedItmes`) _asbp_world_item_base))
          (:`CompletedPin`
            ; UI업데이트 Call
            (`self.OnDroppedItemsUpdate` (`self.CurrentDroppedItmes`))))))))

(fn `UpdateMoveState`
  (params (NewState :type "/Game/Blueprints/Datas/Enum/E_MoveState Enum" :default "NewEnumerator0"))
  (set `self.CurrentMoveState` NewState))

(fn `UpdatePoseState`
  (params (NewPoseState :type "/Game/Blueprints/Datas/Enum/E_PoseState Enum" :default "NewEnumerator0"))
  (set `self.CurrentPoseState` NewPoseState))

(fn `UserConstructionScript`)