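; BP_PlayerController is the player controller that relays movement and look input to the player character.
; On BeginPlay it casts the first player character to BP_Player and caches the reference.
; Its Turn, LookUp, MoveForward and MoveRight axis events forward their values to that character's functions, with both move axes sharing one Move call distinguished by an IsForward flag.
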(event `self.ReceiveBeginPlay`
  (bind _asbp_player (cast `/Game/Blueprints/Character/BP_Player` (`GameplayStatics.GetPlayerCharacter` 0)))
  (set `self.BP Player` _asbp_player))

(event `InputAxis|Turn`
  (params (AxisValue :type "Float (single-precision)"))
  (`/Game/Blueprints/Character/BP_Player.InputTurn` (`self.BP Player`) AxisValue))

(event `InputAxis|MoveForward`
  (params (AxisValue :type "Float (single-precision)"))
  (`/Game/Blueprints/Character/BP_Player.Move` (`self.BP Player`) true AxisValue))

(event `InputAxis|MoveRight`
  (params (AxisValue :type "Float (single-precision)"))
  (`/Game/Blueprints/Character/BP_Player.Move` (`self.BP Player`) false AxisValue))

(event `InputAxis|LookUp`
  (params (AxisValue :type "Float (single-precision)"))
  (`/Game/Blueprints/Character/BP_Player.InputLookUp` (`self.BP Player`) AxisValue))

(fn `UserConstructionScript`)